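; BP_lightball is a spinning light ball actor made of nine sphere components, each tinted a random color.
; On BeginPlay it gathers the spheres into an array and gives each a dynamic instance of M_lightballray with a random "color" parameter.
; Tick advances roll at a slow, frame-rate-independent speed and sets yaw to that same roll-derived value, leaving pitch unchanged.
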(event `self.ReceiveBeginPlay`
  (`KismetArrayLibrary.Array_Add` (`self.NewVar_0`) (`self.Sphere1`))
  (`KismetArrayLibrary.Array_Add` (`self.NewVar_0`) (`self.Sphere2`))
  (`KismetArrayLibrary.Array_Add` (`self.NewVar_0`) (`self.Sphere3`))
  (`KismetArrayLibrary.Array_Add` (`self.NewVar_0`) (`self.Sphere4`))
  (`KismetArrayLibrary.Array_Add` (`self.NewVar_0`) (`self.Sphere5`))
  (`KismetArrayLibrary.Array_Add` (`self.NewVar_0`) (`self.Sphere6`))
  (`KismetArrayLibrary.Array_Add` (`self.NewVar_0`) (`self.Sphere7`))
  (`KismetArrayLibrary.Array_Add` (`self.NewVar_0`) (`self.Sphere8`))
  (`KismetArrayLibrary.Array_Add` (`self.NewVar_0`) (`self.Sphere9`))
  (for _array_element (`self.NewVar_0`)
    (bind _returnvalue (`PrimitiveComponent.CreateDynamicMaterialInstance` _array_element 0 "/Game/Model/lightball/M_lightballray.M_lightballray" "None"))
    (`MaterialInstanceDynamic.SetVectorParameterValue` _returnvalue "color" (make `LinearColor` (`KismetMathLibrary.RandomFloat`) (`KismetMathLibrary.RandomFloat`) (`KismetMathLibrary.RandomFloat`) 1.0))
    (`PrimitiveComponent.SetMaterial` _array_element 0 _returnvalue)))

(event `self.ReceiveTick`
  (params (DeltaSeconds :type "Float (single-precision)"))
  (bind (_returnvalue_roll _returnvalue_pitch) (`KismetMathLibrary.BreakRotator` (`self.K2_GetActorRotation`)))
  (bind _returnvalue (+ _returnvalue_roll (* 5 (`GameplayStatics.GetWorldDeltaSeconds`))))
  (`self.K2_SetActorRotation` (`KismetMathLibrary.MakeRotator` _returnvalue _returnvalue_pitch _returnvalue)))

(fn `UserConstructionScript`)